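; Player controller with top-down click-and-touch movement logic, currently inert because nothing triggers its input chains and Tick is empty.
; The disconnected gated chains trace under the cursor (skipped with a headset enabled) or first finger on the Visibility channel.
; Both feed MoveToHitLocation, which calls SimpleMoveToLocation unless the hit is closer to the pawn than MinClickDistance.
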(event EventTick
  (params (DeltaSeconds :type Float%20%28single-precision%29))
  ;[1 1 1] Click and go there
)

(event Input|TouchEvents|InputTouch
  (params (Location :type Vector) (FingerIndex :type ETouchIndex%20Enum))
  ;[1 1 1] Click and go there
)

(fn ConstructionScript)

(fn MovetoHitLocation
  (params (Hit :type Hit%20Result%20Structure))
  (bind (_bblockinghit _binitialoverlap _time _distance _location _impactpoint) (Collision|BreakHitResult Hit))
  (if (>= (Math|Vector|VectorLength (- (Transformation|GetActorLocation (Pawn|GetControlledPawn)) _location)) (Variables|Default|GetMinClickDistance)) ; Don't move if player clicks too close to pawn
    (AI|Navigation|SimpleMovetoLocation self _location)))